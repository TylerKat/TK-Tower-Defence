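; BP_SpawnPoint is a spawn point that, from BeginPlay, spawns timed waves of BP_Imp enemies at its root location.
; SpawnWave increments WaveNumber, spawns imps one second apart using a LoopCount loop against NumEnmy, then calls itself after a long delay.
; Every tenth wave is meant as a dog wave but only prints a debug string, which ends the wave cycle.
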(event `self.ReceiveBeginPlay`
  (`self.SpawnWave`))

(event `SpawnWave`
  ;[1 1 1] Skip for wave 0 only
  (if (== (`self.WaveNumber`) 0.0)
    (`KismetSystemLibrary.PrintString` "false" :!label _label)
    ;[1 1 1] Imp Spawning code
    (`/Engine/EditorBlueprintResources/StandardMacros.IncrementFloat` (`self.WaveNumber`)
      (:`  `
        (if (<= (`self.LoopCount`) (`self.NumEnmy`)) :!label _label_2
          (`AIBlueprintHelperLibrary.SpawnAIFromClass` "/Game/BluePrints/Enemies/BP_Imp.BP_Imp_C" null (`SceneComponent.K2_GetComponentLocation` (`self.DefaultSceneRoot`)) (struct) false null)
          (`/Engine/EditorBlueprintResources/StandardMacros.IncrementInt` (`self.LoopCount`)
            (:`  `
              (`KismetSystemLibrary.Delay` 1.0)
              (goto _label_2)))
          (else
            (set `self.LoopCount` 0)
            (`KismetSystemLibrary.PrintString` "end of wave")
            (`KismetSystemLibrary.Delay` 150.0)
            (`self.SpawnWave`)))))
    (else
      ;[1 1 1] Check if wave is divisable by 10, if so switch to dog wave
      (if (== (mod (`self.WaveNumber`) 10.0) 0.0)
        (`KismetSystemLibrary.PrintString` "true")
        (else
          (goto _label))))))

(fn `UserConstructionScript`)