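; Player camera character that pans along fixed world axes with the mouse cursor visible, suggesting a top-down view.
; Movement inputs feed CharacterMovement, with held fast and slow actions changing max walk speed and restoring normal on release.
; Mouse wheel steps CurrentZoom to set spring arm height.
; A CanZoom flag flags out-of-range values, so clamping to the limits happens on the following scroll, allowing one step of overshoot.
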(event `self.ReceiveBeginPlay`
  (set `PlayerController.bShowMouseCursor` true (`GameplayStatics.GetPlayerController` 0)))

(event `InputAxis|Move RightLeft`
  (params (AxisValue :type "Float (single-precision)"))
  ;[1 1 1] Player Movement
  (`self.AddMovementInput` (1.0 0.0 0.0) AxisValue))

(event `InputAction|FastMovement`
  (params (Key :type "Key Structure"))
  (bind _charactermovement (`self.CharacterMovement`))
  ;[1 1 1] Sprint/slow
  (:`Pressed`
    (set `CharacterMovementComponent.MaxWalkSpeed` 2400.0 _charactermovement) ; Set Fast speed
  )
  (:`Released`
    (set `CharacterMovementComponent.MaxWalkSpeed` 1200.0 _charactermovement :!label _label) ; Set to normal speed
  ))

(event `InputAxis|Move frontback`
  (params (AxisValue :type "Float (single-precision)"))
  ;[1 1 1] Player Movement
  (`self.AddMovementInput` (0.0 -1.0 0.0) AxisValue))

(event `InputAction|SlowMovement`
  (params (Key :type "Key Structure"))
  ;[1 1 1] Sprint/slow
  (:`Pressed`
    (set `CharacterMovementComponent.MaxWalkSpeed` 600.0 (`self.CharacterMovement`)) ; Set to slow speed
  )
  (:`Released`
    (goto _label)))

(event `Key|MouseScrollUp`
  (params (Key :type "Key Structure"))
  (bind _currentzoom (`self.CurrentZoom`))
  (bind _returnvalue (<= _currentzoom 1500.0))
  (bind _returnvalue_2 (>= _currentzoom 900.0))
  ;[1 1 1] Camera Zoom
  (:`Pressed`
    (set `self.CurrentZoom` (- (`self.CurrentZoom`) 20.0)) ; Subtracts height
    (if (`self.CanZoom`) :!label _label_2
      (if (not (and _returnvalue _returnvalue_2))
        (set `self.CanZoom` false) ; if not in range then can zoom false
      )
      (elif _returnvalue
        (if (not _returnvalue_2)
          (set `self.CurrentZoom` 900.0) ; Set height to min value
          (set `self.CanZoom` true) ; Can zoom to true
        )
        (else
          (set `self.CurrentZoom` 1500.0) ; sets height to max value
          (set `self.CanZoom` true) ; can zoom to true
        )))
    (`SceneComponent.K2_SetRelativeLocation` (`self.SpringArm`) (`KismetMathLibrary.MakeVector` 0.0 0.0 (`self.CurrentZoom`)) false false) ; Changes the height of spring arm
  ))

(event `Key|MouseScrollDown`
  (params (Key :type "Key Structure"))
  ;[1 1 1] Camera Zoom
  (:`Pressed`
    (set `self.CurrentZoom` (+ (`self.CurrentZoom`) 20.0)) ; Adds height
    (goto _label_2)))

(fn `UserConstructionScript`)