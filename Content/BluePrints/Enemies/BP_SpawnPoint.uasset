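; Enemy spawn point that runs endless numbered waves, spawning AI at its own location one per second.
; SpawnWave increments the wave, grows the enemy count through AmountSpawn, loops the spawns, then calls itself after a long delay.
; Waves spawn imps, except when the pre-increment number is a nonzero multiple of ten, which spawns BP_BaseEnemy as a dog wave.
; AmountSpawn adds to the running count from a table indexed by wave modulo 40.
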(event `SpawnWave`
  ;[1 1 1] Skip for wave 0 only
  (if (== (`self.WaveNumber`) 0)
    ;[1 1 1] Imp Spawning code
    (`/Engine/EditorBlueprintResources/StandardMacros.IncrementInt` (`self.WaveNumber`) :!label _label
      (:`  `
        (`self.AmountSpawn`)
        (if (<= (`self.LoopCount`) (`self.NumEnmy`)) :!label _label_2
          (`AIBlueprintHelperLibrary.SpawnAIFromClass` "/Game/BluePrints/Enemies/BP_Enemy_IMP.BP_Enemy_IMP_C" null (`SceneComponent.K2_GetComponentLocation` (`self.DefaultSceneRoot`)) (struct) false null)
          (`/Engine/EditorBlueprintResources/StandardMacros.IncrementInt` (`self.TotalNumOfEnemies`)
            (:`  `
              (`/Engine/EditorBlueprintResources/StandardMacros.IncrementInt` (`self.LoopCount`)
                (:`  `
                  (`KismetSystemLibrary.Delay` 1.0)
                  (goto _label_2)))))
          (else
            (set `self.LoopCount` 1)
            (`KismetSystemLibrary.PrintString` "end of wave")
            (`KismetSystemLibrary.Delay` 150.0)
            (`self.SpawnWave`)))))
    (else
      ;[1 1 1] Check if wave is divisable by 10, if so switch to dog wave
      (if (== (mod (`self.WaveNumber`) 10) 0)
        ;[1 1 1] Dog Waves
        (`/Engine/EditorBlueprintResources/StandardMacros.IncrementInt` (`self.WaveNumber`)
          (:`  `
            (`self.AmountSpawn`)
            (if (<= (`self.LoopCount`) (`self.NumEnmy`)) :!label _label_3
              (`AIBlueprintHelperLibrary.SpawnAIFromClass` "/Game/BluePrints/Enemies/BP_BaseEnemy.BP_BaseEnemy_C" null (`SceneComponent.K2_GetComponentLocation` (`self.DefaultSceneRoot`)) (struct) false null)
              (`/Engine/EditorBlueprintResources/StandardMacros.IncrementInt` (`self.TotalNumOfEnemies`)
                (:`  `
                  (`/Engine/EditorBlueprintResources/StandardMacros.IncrementInt` (`self.LoopCount`)
                    (:`  `
                      (`KismetSystemLibrary.Delay` 1.0)
                      (goto _label_3)))))
              (else
                (set `self.LoopCount` 1)
                (`KismetSystemLibrary.PrintString` "end of wave")
                (`KismetSystemLibrary.Delay` 150.0)
                (`self.SpawnWave`)))))
        (else
          (goto _label))))))

(event `AmountSpawn`
  ;[1 1 1] Wave index, deturmin enemies that should span base off of wave number
  (set `self.NumEnmy` (+ (`self.NumEnmy`) (select `int` (mod (`self.WaveNumber`) 40) :`0` 100 :`1` 10 :`2` 20 :`3` 25 :`4` 30 :`5` 35 :`6` 40 :`7` 45 :`8` 50 :`9` 50 :`10` 25 :`11` 55 :`12` 60 :`13` 80 :`14` 80 :`15` 80 :`16` 0 :`17` 0 :`18` 0 :`19` 0 :`20` 0 :`21` 0 :`22` 0 :`23` 0 :`24` 0 :`25` 0 :`26` 0 :`27` 0 :`28` 0 :`29` 0 :`30` 0 :`31` 0 :`32` 0 :`33` 0 :`34` 0 :`35` 0 :`36` 0 :`37` 0 :`38` 0 :`39` 0))))

(fn `UserConstructionScript`)