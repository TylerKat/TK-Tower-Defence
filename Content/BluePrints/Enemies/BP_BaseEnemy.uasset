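; Base tower-defense enemy that walks a track of Bp_trackPoint actors, damaging the player's life if it reaches the end.
; BeginPlay gathers the points, and AIMoveTo visits them by array index, re-issuing every 0.2 seconds, up to a hard-coded last index.
; TakeDamge updates the health widget; death awards money and decrements BP_SpawnPoint's enemy count.
; Enemies reaching the end are destroyed without decrementing that count.
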(event `self.ReceiveBeginPlay`
  ;[1 1 1] Refrence to track
  (bind _outactors (`GameplayStatics.GetAllActorsOfClass` "/Game/BluePrints/Enemies/Bp_trackPoint.Bp_trackPoint_C"))
  (set `self.TrackPointArray` _outactors)
  (`self.Move to point`))

(event `Move to point`
  ;[1 1 1] Move along track
  (`|AIMoveTo` self (0.0 0.0 0.0) (`|GetArrayItem` (`self.TrackPointArray`) (`self.PointNumber`)) :!label _label
    (:`then`
      (`KismetSystemLibrary.Delay` 0.2 :!label _label_2)
      (goto _label))
    (:`OnSuccess`
      (`/Engine/EditorBlueprintResources/StandardMacros.IncrementInt` (`self.PointNumber`)
        (:`  `
          (if (> (`self.PointNumber`) 11)
            (bind _asbp_player_cmera (cast `/Game/BluePrints/Player/BP_PlayerCmera` (`GameplayStatics.GetPlayerCharacter` 0)))
            (`/Game/BluePrints/Player/BP_PlayerCmera.RemoveLife` _asbp_player_cmera (`self.Damage`)) ; removes life from player, code in player
            (`self.K2_DestroyActor`)
            (else
              (`self.Move to point`))))))
    (:`OnFail`
      (goto _label_2))))

(event `Take Damge`
  (params (Damage :type "Float (double-precision)"))
  ;[1 1 1] Tower hit enemy code
  (set `self.CurrentHealth` (- (`self.CurrentHealth`) Damage))
  (bind _asw_enemy_health (cast `/Game/BluePrints/HUDS/W_EnemyHealth` (`WidgetComponent.GetUserWidgetObject` (`self.Health`))))
  (`/Game/BluePrints/HUDS/W_EnemyHealth.UpdateHealthBar` _asw_enemy_health (`self.CurrentHealth`) (`self.MaxHealth`))
  (if (<= (`self.CurrentHealth`) 0.0)
    (bind _asbp_player_cmera (cast `/Game/BluePrints/Player/BP_PlayerCmera` (`GameplayStatics.GetPlayerCharacter` 0)))
    (`/Game/BluePrints/Player/BP_PlayerCmera.AddMoney` _asbp_player_cmera (`self.MoneyValue`)) ; add money to player, code in player
    (bind _outactors (`GameplayStatics.GetAllActorsOfClass` "/Game/BluePrints/Enemies/BP_SpawnPoint.BP_SpawnPoint_C"))
    (`/Engine/EditorBlueprintResources/StandardMacros.DecrementInt` (`/Game/BluePrints/Enemies/BP_SpawnPoint.TotalNumOfEnemies` (`|GetArrayItem` _outactors)) ; decrease number of enemies counter
      (:`  `
        (`self.K2_DestroyActor`)))))

(fn `UserConstructionScript`)