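; BP_Imp is an enemy that walks a track of Bp_trackPoint actors and destroys itself at the end.
; On BeginPlay it gathers all track points with GetAllActorsOfClass, using the returned order as the route without sorting.
; MoveToPoint runs AIMoveTo to the current point, then increments the index and calls itself on success.
; The track end is a hardcoded index, and failed moves are not handled.
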(event `self.ReceiveBeginPlay`
  ;[1 1 1] Refrence to track
  (bind _outactors (`GameplayStatics.GetAllActorsOfClass` "/Game/BluePrints/Bp_trackPoint.Bp_trackPoint_C"))
  (set `self.TrackPointArray` _outactors)
  (`self.Move to point`))

(event `Move to point`
  (bind _output (`|GetArrayItem` (`self.TrackPointArray`) (`self.PointNumber`)))
  ;[1 1 1] Move along track
  (`|AIMoveTo` self (0.0 0.0 0.0) _output
    (:`OnSuccess`
      (`KismetSystemLibrary.PrintString` (`KismetSystemLibrary.GetDisplayName` _output))
      (`/Engine/EditorBlueprintResources/StandardMacros.IncrementInt` (`self.PointNumber`)
        (:`  `
          (if (> (`self.PointNumber`) 11)
            (`KismetSystemLibrary.PrintString` "Done")
            (`self.K2_DestroyActor`)
            (else
              (`self.Move to point`))))))))

(fn `UserConstructionScript`)