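; Base tower projectile that homes in on an enemy and deals damage on overlap.
; HomingAttack stores the target, damage, attack type and money multiplier, sets the homing component and destroys the projectile after a timeout.
; Overlap damages whichever enemy is hit, but applies the slow-or-speed update or poison effect to the stored target before destroying itself.
; Tick removes the projectile once its target becomes invalid.
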(event `HomingAttack`
  (params (Enemy :type "/Game/BluePrints/Enemies/BP_BaseEnemy Object Reference") (Damage :type "Float (double-precision)") (AttackType :type Integer) (MultiplierMoney :type "Float (double-precision)"))
  ;[1 1 1] Get damage, target, and attack type
  (set `self.Multiplier Money` MultiplierMoney) ; Come from tower base
  (set `self.Enemy` Enemy)
  (set `self.Damage` Damage)
  (set `self.Attack Type` AttackType)
  (set `ProjectileMovementComponent.HomingTargetComponent` (`SceneComponent.GetChildComponent` (`Character.CapsuleComponent` Enemy) 0) (`self.ProjectileMovement`))
  (`KismetSystemLibrary.Delay` 20.0)
  (`self.K2_DestroyActor`))

(event `self.Collision.OnComponentBeginOverlap`
  (params (OverlappedComponent :type "PrimitiveComponent Object Reference") (OtherActor :type "Actor Object Reference") (OtherComp :type "PrimitiveComponent Object Reference") (OtherBodyIndex :type Integer) (bFromSweep :type Boolean) (SweepResult :type "HitResult Structure (by ref)"))
  (bind _enemy (`self.Enemy`))
  ;[1 1 1] Apply Damage and extra effects
  (bind _asbp_base_enemy (cast `/Game/BluePrints/Enemies/BP_BaseEnemy` OtherActor))
  (`/Game/BluePrints/Enemies/BP_BaseEnemy.Take Damge` _asbp_base_enemy (`self.Damage`) (`self.Multiplier Money`))
  (if (`KismetSystemLibrary.IsValid` (`self.Enemy`))
    (switch `int` (`self.Attack Type`) ; add extra effect
      (:`Default`
        _)
      (:`0`
        _)
      (:`1`
        (`/Game/BluePrints/Enemies/BP_BaseEnemy.UpdateSpeed` _enemy))
      (:`2`
        (`/Game/BluePrints/Enemies/BP_BaseEnemy.Poisoned` _enemy)))
    (`self.K2_DestroyActor`)))

(event `self.ReceiveTick`
  (params (DeltaSeconds :type "Float (single-precision)"))
  ;[1 1 1] Target is still valid if not remove projectile
  (if (not (`KismetSystemLibrary.IsValid` (`self.Enemy`)))
    (`self.K2_DestroyActor`)))

(fn `UserConstructionScript`)