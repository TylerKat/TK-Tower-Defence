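; Base tower Blueprint for a tower defense game that shoots homing projectiles at enemies in range.
; Range overlaps maintain the enemy list, while Tick uses a Delay cooldown to fire at the first enemy, or all with MultiAttack.
; BeginPlay caches the player camera and creates an upgrade widget linked to the tower.
; Selection events toggle the range indicator and that widget, and MoneyChange increases player money by a multiplier.
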(event `TowerSelected`
  ;[1 1 1] Selecting and deselecting code
  (`SceneComponent.SetVisibility` (`self.N_SelectedTowerRange`) true false)
  (`/Game/BluePrints/Player/BP_PlayerCmera.Remove Widget` (`self.Ref to player`) (`self.MyUpgrades`)))

(event `Tower Deselected`
  ;[1 1 1] Selecting and deselecting code
  (`SceneComponent.SetVisibility` (`self.N_SelectedTowerRange`) false false)
  (`/Game/BluePrints/Player/BP_PlayerCmera.Add Widget` (`self.Ref to player`) (`self.MyUpgrades`)))

(event `self.ReceiveBeginPlay`
  ;[1 1 1] ref to player
  (bind _outactors (`GameplayStatics.GetAllActorsOfClass` "/Game/BluePrints/Player/BP_PlayerCmera.BP_PlayerCmera_C"))
  (set `self.Ref to player` (`|GetArrayItem` _outactors))
  (bind _returnvalue (`|CreateWidget` (`self.Tower Widget`)))
  (bind _output_get (set `self.MyUpgrades` _returnvalue))
  (bind _asw_upgrade_base_tower (cast `/Game/BluePrints/HUDS/TowerUpgradePaths/W_UpgradeBaseTower` _output_get))
  (`/Game/BluePrints/HUDS/TowerUpgradePaths/W_UpgradeBaseTower.Ref To Tower` _asw_upgrade_base_tower self))

(event `self.TowerRange.OnComponentBeginOverlap`
  (params (OverlappedComponent :type "PrimitiveComponent Object Reference") (OtherActor :type "Actor Object Reference") (OtherComp :type "PrimitiveComponent Object Reference") (OtherBodyIndex :type Integer) (bFromSweep :type Boolean) (SweepResult :type "HitResult Structure (by ref)"))
  (bind _enemylist (`self.EnemyLIst`))
  ;[1 1 1] Adds enemy to array and sets in range to true
  (bind _asbp_base_enemy (cast `/Game/BluePrints/Enemies/BP_BaseEnemy` OtherActor))
  (if (not (`KismetArrayLibrary.Array_Contains` _enemylist _asbp_base_enemy))
    (`KismetArrayLibrary.Array_Insert` _enemylist _asbp_base_enemy (+ (`KismetArrayLibrary.Array_LastIndex` _enemylist) 1)) ; insert new enemy into last index in array
    (set `self.InRange` true)))

(event `self.TowerRange.OnComponentEndOverlap`
  (params (OverlappedComponent :type "PrimitiveComponent Object Reference") (OtherActor :type "Actor Object Reference") (OtherComp :type "PrimitiveComponent Object Reference") (OtherBodyIndex :type Integer))
  (bind _enemylist (`self.EnemyLIst`))
  ;[1 1 1] Removes enemies from array and when array in empty set in range to false
  (bind _asbp_base_enemy (cast `/Game/BluePrints/Enemies/BP_BaseEnemy` OtherActor))
  (`KismetArrayLibrary.Array_Remove` _enemylist (`KismetArrayLibrary.Array_Find` _enemylist _asbp_base_enemy))
  (if (<= (`KismetArrayLibrary.Array_Length` (`self.EnemyLIst`)) 0)
    (set `self.InRange` false)))

(event `self.ReceiveTick`
  (params (DeltaSeconds :type "Float (single-precision)"))
  (bind _enemylist (`self.EnemyLIst`))
  (bind (_returnvalue_location _returnvalue_rotation) (`KismetMathLibrary.BreakTransform` (`SceneComponent.K2_GetComponentToWorld` (`self.ProSpawnPoint`))))
  ;[1 1 1] Shooting code
  (if (`self.InRange`)
    (`KismetSystemLibrary.Delay` (`self.CoolDown`)) ; cooldown on fire rate
    (if (`self.MultiAttack`)
      (`self.TargetAll`)
      (elif (`KismetArrayLibrary.Array_Contains` _enemylist (`|GetArrayItem` _enemylist))
        (bind _returnvalue (`|SpawnActorFromClass` "/Game/BluePrints/Projectiles/BP_projectileBase.BP_projectileBase_C" (`KismetMathLibrary.MakeTransform` _returnvalue_location _returnvalue_rotation) "AlwaysSpawn" "MultiplyWithRoot" null null))
        (`/Game/BluePrints/Projectiles/BP_projectileBase.HomingAttack` _returnvalue (`|GetArrayItem` (`self.EnemyLIst`)) (`self.Damage`) (`self.Attack Type`))))))

(event `MoneyChange`
  (`/Game/BluePrints/Player/BP_PlayerCmera.IncreaseMoney` (`self.Ref to player`) (`self.Multiplier`)))

(event `TargetAll`
  (bind (_returnvalue_location _returnvalue_rotation) (`KismetMathLibrary.BreakTransform` (`SceneComponent.K2_GetComponentToWorld` (`self.ProSpawnPoint`))))
  (for (_ _array_index) (`self.EnemyLIst`)
    (bind _returnvalue (`|SpawnActorFromClass` "/Game/BluePrints/Projectiles/BP_projectileBase.BP_projectileBase_C" (`KismetMathLibrary.MakeTransform` _returnvalue_location _returnvalue_rotation) "AlwaysSpawn" "MultiplyWithRoot" null null))
    (`/Game/BluePrints/Projectiles/BP_projectileBase.HomingAttack` _returnvalue (`|GetArrayItem` (`self.EnemyLIst`) _array_index) (`self.Damage`) (`self.Attack Type`))))

(fn `UserConstructionScript`)