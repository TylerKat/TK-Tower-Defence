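; BP_Tower-5 is a tower variant that trades per-hit damage and attack rate for multi-attack.
; On BeginPlay it runs the parent logic, then halves Damage, enables MultiAttack and lengthens CoolDown by scaling the inherited values.
; It adds no attack logic of its own, leaving that to the parent class, and its construction script only calls the parent.
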(event `self.ReceiveBeginPlay`
  (`parent.ReceiveBeginPlay`)
  (set `self.Damage` (/ (`self.Damage`) 2.0))
  (set `self.MultiAttack` true)
  (set `self.CoolDown` (* (`self.CoolDown`) 1.5)))

(fn `UserConstructionScript`
  (`parent.UserConstructionScript`))