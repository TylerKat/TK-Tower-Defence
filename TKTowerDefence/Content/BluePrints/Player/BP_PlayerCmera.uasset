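; Player camera pawn that moves along fixed world axes and zooms with the mouse wheel.
; Two axis inputs feed movement input along world X and negative Y.
; Wheel presses print debug text and step CurrentZoom, which sets the spring arm's relative Z height, not its arm length, when CanZoom is true.
; The range checks meant to update CanZoom are unconnected, so CurrentZoom changes without limits.
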(event `InputAxis|Move RightLeft`
  (params (AxisValue :type "Float (single-precision)"))
  ;[1 1 1] Player Movement
  (`self.AddMovementInput` (1.0 0.0 0.0) AxisValue))

(event `InputAxis|Move frontback`
  (params (AxisValue :type "Float (single-precision)"))
  ;[1 1 1] Player Movement
  (`self.AddMovementInput` (0.0 -1.0 0.0) AxisValue))

(event `Key|MouseScrollUp`
  (params (Key :type "Key Structure"))
  (:`Pressed`
    (`KismetSystemLibrary.PrintString` "Hello")
    (set `self.CurrentZoom` (- (`self.CurrentZoom`) 10.0))
    (if (`self.CanZoom`) :!label _label
      (`SceneComponent.K2_SetRelativeLocation` (`self.SpringArm`) (`KismetMathLibrary.MakeVector` 0.0 0.0 (`self.CurrentZoom`)) false false))))

(event `Key|MouseScrollDown`
  (params (Key :type "Key Structure"))
  (:`Pressed`
    (`KismetSystemLibrary.PrintString` "bye")
    (set `self.CurrentZoom` (+ (`self.CurrentZoom`) 10.0))
    (goto _label)))

(fn `UserConstructionScript`)